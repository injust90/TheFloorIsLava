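; BP_BrickSpawner is an actor that spawns a row of four BP_Bricks actors for a brick breaker game when play begins.
; A BeginPlay loop places each brick at a fixed step along world Y from the spawner's location, using the spawner's rotation and unit scale.
; The spacing does not follow the spawner's rotation, and the construction script, overlap and tick events do nothing.
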(event `self.ReceiveBeginPlay`
  (for _index (range 4)
    (`|SpawnActorFromClass` "/Game/BrickBreakerAssets/BP_Bricks.BP_Bricks_C" (`KismetMathLibrary.MakeTransform` (+ (* (`KismetMathLibrary.Conv_IntVectorToVector` (make `IntVector` 0 _index)) (0.0 700.0 0.0)) (`self.K2_GetActorLocation`)) (`self.K2_GetActorRotation`)) "Undefined" "MultiplyWithRoot" null null)))

(fn `UserConstructionScript`)