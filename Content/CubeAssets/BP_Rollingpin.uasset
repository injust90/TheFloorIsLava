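; BP_Rollingpin is a moving actor whose Cube component slides back and forth along its local Y axis.
; A timeline started on BeginPlay drives both relative Y position and yaw from one track, without sweep, and prints the position each update.
; The update also feeds a three-second Delay, after which the IsLooped flag toggles the timeline between play and reverse, rather than using its Finished output.
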(event `self.ReceiveBeginPlay`
  (bind (_direction _moving _newtrack_0) (`Timeline|Timeline` :!label _label)
    (:`Update`
      (bind _returnvalue (`KismetMathLibrary.MakeVector` 0.0 _newtrack_0))
      (`KismetSystemLibrary.PrintString` (`KismetStringLibrary.Conv_VectorToString` _returnvalue))
      (`SceneComponent.K2_SetRelativeLocation` (`self.Cube`) _returnvalue false false)
      (`SceneComponent.K2_SetRelativeRotation` (`self.Cube`) (`KismetMathLibrary.MakeRotator` 0.0 0.0 _newtrack_0) false false)
      (`KismetSystemLibrary.Delay` 3.0)
      (if (`self.IsLooped`)
        (set `self.IsLooped` false)
        (goto _label)
        (else
          (set `self.IsLooped` true)
          (goto _label :!via `Reverse`))))))

(fn `UserConstructionScript`
  (`parent.UserConstructionScript`))