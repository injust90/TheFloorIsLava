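; BP_WinCircle is a goal trigger that ends the level in a win when the third-person character overlaps it.
; On overlap it sets its text render to a win message and switches the material on its four static meshes.
; It also finds the CountDownTimer widgets through GetAllWidgetsOfClass and calls TimerStateMessage on them.
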(event `self.ReceiveActorBeginOverlap`
  (params (OtherActor :type "Actor Object Reference"))
  (cast `/Game/ThirdPerson/Blueprints/BP_ThirdPersonCharacter` OtherActor)
  (`TextRenderComponent.K2_SetText` (`self.TextRender`) (`KismetTextLibrary.Conv_StringToText` "You win!"))
  (bind _foundwidgets (`WidgetBlueprintLibrary.GetAllWidgetsOfClass` "/Game/CubeAssets/CountDownTimer.CountDownTimer_C" false))
  (message `/Game/CubeAssets/BPI_Pause.Timer State` _foundwidgets true)
  (`PrimitiveComponent.SetMaterial` (`self.StaticMesh`) 0 "/Game/CustomMaterials/MMI_WinCircle.MMI_WinCircle")
  (`PrimitiveComponent.SetMaterial` (`self.StaticMesh1`) 0 "/Game/CustomMaterials/MMI_WinCircle.MMI_WinCircle")
  (`PrimitiveComponent.SetMaterial` (`self.StaticMesh2`) 0 "/Game/CustomMaterials/MMI_WinCircle.MMI_WinCircle")
  (`PrimitiveComponent.SetMaterial` (`self.StaticMesh3`) 0 "/Game/CustomMaterials/MMI_WinCircle.MMI_WinCircle"))

(fn `UserConstructionScript`)