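; BP_Wall is a wall actor that damages the BallPawn when it hits fast enough.
; On begin overlap it casts the other actor to BallPawn, prints its velocity, and calls Damage if any velocity axis reaches a fixed threshold.
; The check uses signed per-axis values rather than speed magnitude, so movement in negative directions alone never triggers damage.
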(event `self.ReceiveActorBeginOverlap`
  (params (OtherActor :type "Actor Object Reference"))
  (bind _asball_pawn (cast `/Game/ThirdPerson/Blueprints/BallPawn` OtherActor))
  (`KismetSystemLibrary.PrintString` (`KismetStringLibrary.Conv_VectorToString` (`self.GetVelocity` _asball_pawn)))
  (bind (_returnvalue_x _returnvalue_y _returnvalue_z) (`KismetMathLibrary.BreakVector` (`self.GetVelocity` _asball_pawn)))
  (if (or (>= _returnvalue_x 350.0) (>= _returnvalue_y 350.0) (>= _returnvalue_z 350.0))
    (`/Game/ThirdPerson/Blueprints/BallPawn.Damage` _asball_pawn)))

(fn `UserConstructionScript`)