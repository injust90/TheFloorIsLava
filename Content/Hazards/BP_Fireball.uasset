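; BP_Fireball is a hazard whose sphere moves vertically and sends the player back on contact.
; A Timeline drives the sphere's relative Z, with a three-second Delay on its Update pin toggling IsLooped to alternate Play and Reverse.
; On actor overlap, it moves BP_ThirdPersonCharacter to that character's stored Location and calls TimerRestartMessage on the CountDownTimer widgets.
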(event `self.ReceiveBeginPlay`
  (bind (_direction _moving _newtrack_0) (`Timeline|Timeline` :!label _label)
    (:`Update`
      (`SceneComponent.K2_SetRelativeLocation` (`self.Sphere`) (`KismetMathLibrary.MakeVector` 0.0 0.0 _newtrack_0) false false)
      (`KismetSystemLibrary.Delay` 3.0)
      (if (`self.IsLooped`)
        (set `self.IsLooped` false)
        (goto _label)
        (else
          (set `self.IsLooped` true)
          (goto _label :!via `Reverse`))))))

(event `self.ReceiveActorBeginOverlap`
  (params (OtherActor :type "Actor Object Reference"))
  (bind _asbp_third_person_character (cast `/Game/ThirdPerson/Blueprints/BP_ThirdPersonCharacter` OtherActor))
  (`self.K2_SetActorLocation` _asbp_third_person_character (`/Game/ThirdPerson/Blueprints/BP_ThirdPersonCharacter.Location` _asbp_third_person_character) false false)
  (bind _foundwidgets (`WidgetBlueprintLibrary.GetAllWidgetsOfClass` "/Game/CubeAssets/CountDownTimer.CountDownTimer_C"))
  (message `/Game/CubeAssets/BPI_Pause.Timer Restart` _foundwidgets))

(fn `UserConstructionScript`)